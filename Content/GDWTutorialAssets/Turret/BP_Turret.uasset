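; Turret actor that spots the player with AI Perception sight, tracks them and fires a laser that deals damage.
; Sensing a Player-tagged actor starts two looping timers: one smoothly turns the head toward the target, the other fires.
; Each shot spawns a Niagara beam and line-traces forward, applying damage through BPI_Character.
; Forgetting the player stops both timers, and enable/disable events toggle the sight sense.
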(event `self.ReceiveBeginPlay`
  ; Disable Turret if Enabled is not True on Start
  (if (not (`self.Enabled`))
    (`self.Event OnDisableTurret`)))

(event `Event OnEnableTurret`
  (bind _aiperception (`self.AIPerception`))
  ; Enable Turret Senses
  (set `self.Enabled` true)
  (`AIPerceptionComponent.SetSenseEnabled` _aiperception "/Script/AIModule.AISense_Sight" true)
  (`AIPerceptionComponent.ForgetAll` _aiperception))

(event `self.AIPerception.OnTargetPerceptionUpdated`
  (params (Actor :type "Actor Object Reference") (Stimulus :type "AIStimulus Structure"))
  ; Use AI Perception to "See" the Player
  (`self.TurretTarget`
    (:`then`)
    (:`else`
      (`KismetSystemLibrary.PrintString` "Percieved Target!")
      (if (and (`self.ActorHasTag` Actor "Player") (`.bSuccessfullySensed` (break `AIStimulus` Stimulus)))
        (set `self.TurretTarget` Actor)
        (`self.Event TrackTarget`)))))

(event `Event TrackTarget`
  ; Set Tracking and Shooting Timer Loops
  (bind _returnvalue (`KismetSystemLibrary.K2_SetTimerDelegate` (delegate `Event MoveTurret`) 0.03 true true))
  (set `self.TrackTimer` _returnvalue)
  (bind _returnvalue_2 (`KismetSystemLibrary.K2_SetTimerDelegate` (delegate `Event ShootTarget`) (`self.ShootingSpeed`) true true))
  (set `self.ShootTimer` _returnvalue_2))

(event `Event MoveTurret`
  (bind _turrethead (`self.TurretHead`))
  ; Rotate Turret Toward Target
  (bind _turrettarget (`self.TurretTarget`)
    (:`then`
      (bind (_returnvalue_roll _returnvalue_pitch _returnvalue_yaw) (`KismetMathLibrary.BreakRotator` (`KismetMathLibrary.RInterpTo` (`SceneComponent.K2_GetComponentRotation` _turrethead) (`KismetMathLibrary.FindLookAtRotation` (`SceneComponent.K2_GetComponentLocation` _turrethead) (`self.K2_GetActorLocation` _turrettarget)) (`GameplayStatics.GetWorldDeltaSeconds`) (`self.TurnSpeed`))))
      (`SceneComponent.K2_SetWorldRotation` _turrethead (`KismetMathLibrary.MakeRotator` 0.0 _returnvalue_pitch _returnvalue_yaw) false false))
    (:`else`)))

(event `Event ShootTarget`
  (bind _shootpoint (`self.ShootPoint`))
  (bind (_returnvalue_location _returnvalue_rotation) (`KismetMathLibrary.BreakTransform` (`SceneComponent.K2_GetComponentToWorld` (`self.ShootPoint`))))
  (bind _returnvalue (`SceneComponent.K2_GetComponentLocation` _shootpoint))
  ; Shoot At Player
  (bind _returnvalue_2 (`NiagaraFunctionLibrary.SpawnSystemAtLocation` "/Game/GDWTutorialAssets/Turret/VFX/NS_TurretLaser.NS_TurretLaser" _returnvalue_location _returnvalue_rotation (1.0 1.0 1.0) true false "AutoRelease"))
  (bind _turrettarget (`self.TurretTarget`)
    (:`then`
      (`NiagaraComponent.SetVariableVec3` _returnvalue_2 "BeamLength" (`KismetMathLibrary.MakeVector` (`KismetMathLibrary.Vector_Distance` _returnvalue_location (`self.K2_GetActorLocation` _turrettarget))))
      (`ActorComponent.Activate` _returnvalue_2 true)
      (bind (_outhit _returnvalue_3) (`KismetSystemLibrary.LineTraceSingle` :`Start` _returnvalue :`End` (+ _returnvalue (* (`SceneComponent.GetForwardVector` _shootpoint) (`self.ShootRange`))) :`TraceChannel` "TraceTypeQuery2" :`DrawDebugType` "ForDuration"))
      (if _returnvalue_3
        (if (`self.ActorHasTag` (`.HitActor` (`GameplayStatics.BreakHitResult` _outhit)) "Player")
          (if (`KismetSystemLibrary.DoesImplementInterface` (`.HitActor` (`GameplayStatics.BreakHitResult` _outhit)) "/Game/GDWTutorialAssets/Interfaces/BPI_Character.BPI_Character_C")
            (bind _asbpi_character (cast `/Game/GDWTutorialAssets/Interfaces/BPI_Character` (`.HitActor` (`GameplayStatics.BreakHitResult` _outhit))))
            (`/Game/GDWTutorialAssets/Interfaces/BPI_Character.UpdateHealth` _asbpi_character (`self.TurretDamage`) self)))))
    (:`else`)))

(event `self.AIPerception.OnTargetPerceptionForgotten`
  (params (Actor :type "Actor Object Reference"))
  ; Stop Timer Loops When Target Leaves Range
  (`/Engine/EditorBlueprintResources/StandardMacros.IsValid` Actor
    (:`Is Valid`
      (if (`self.ActorHasTag` Actor "Player")
        (`self.TurretTarget`
          (:`then`
            (`KismetSystemLibrary.K2_ClearAndInvalidateTimerHandle` (`self.TrackTimer`))
            (`KismetSystemLibrary.K2_ClearAndInvalidateTimerHandle` (`self.ShootTimer`))
            (set `self.TurretTarget` null))
          (:`else`))))))

(event `Event OnDisableTurret`
  (bind _aiperception (`self.AIPerception`))
  ; Disable Turret Senses, Forget All Percieved Targets, and Disable Looping Timers
  (set `self.Enabled` false)
  (`AIPerceptionComponent.SetSenseEnabled` _aiperception "/Script/AIModule.AISense_Sight" false)
  (`AIPerceptionComponent.ForgetAll` _aiperception)
  (`KismetSystemLibrary.K2_ClearAndInvalidateTimerHandle` (`self.TrackTimer`))
  (`KismetSystemLibrary.K2_ClearAndInvalidateTimerHandle` (`self.ShootTimer`))
  (set `self.TurretTarget` null))

(fn `UserConstructionScript`)